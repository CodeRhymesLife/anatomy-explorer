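; Organ actor that displays an assigned mesh and computes a palm placement from Leap Motion hand data.
; On BeginPlay it applies the Mesh variable to its OrganContainer component.
; GetPalmPositionAndOrientation projects forward from the player character by a multiple of forearm length, plus a height offset, using the oldest hand on the grab side.
; Tracked bone positions are zeroed out, and orientation is the forearm's, doubled.
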(event `self.ReceiveBeginPlay`
  (`StaticMeshComponent.SetStaticMesh` (`self.organContainer`) (`self.mesh`)))

(fn `UserConstructionScript`)