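; Quiz question actor that shows organ-type answer options on four text components.
; On BeginPlay it labels each component from the OrganTypeOptions enum array, prefixing every name with a dash.
; Only Option1 reacts to overlap, switching to the Correct material on begin and back to DefaultMat on end, so the correct answer is fixed to that slot.
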(event `self.ReceiveBeginPlay`
  (set `self.organTextElements` (`|MakeArray` (`self.option1`) (`self.option2`) (`self.option3`) (`self.option4`)))
  (for (_array_element _array_index) (`self.organTypeOptions`)
    (`TextRenderComponent.K2_SetText` (`KismetArrayLibrary.Array_Get` (`self.organTextElements`) _array_index) (`KismetTextLibrary.Conv_StringToText` (`KismetStringLibrary.Concat_StrStr` "- " (`|GetEnumeratorNameAsString` _array_element))))))

(event `self.ReceiveActorBeginOverlap`
  (params (OtherActor :type "Actor Object Reference")))

(event `self.ReceiveTick`
  (params (DeltaSeconds :type "Float (single-precision)")))

(event `self.option1.OnComponentBeginOverlap`
  (params (OtherActor :type "Actor Object Reference") (OtherComp :type "PrimitiveComponent Object Reference") (OtherBodyIndex :type Integer) (bFromSweep :type Boolean) (SweepResult :type "HitResult Structure (by ref)"))
  (`PrimitiveComponent.SetMaterial` (`self.option1`) 0 "/Game/Materials/correct.correct"))

(event `self.option1.OnComponentEndOverlap`
  (params (OtherActor :type "Actor Object Reference") (OtherComp :type "PrimitiveComponent Object Reference") (OtherBodyIndex :type Integer))
  (`PrimitiveComponent.SetMaterial` (`self.option1`) 0 "/Game/modified/defaultMat.defaultMat"))

(fn `UserConstructionScript`)