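; Leap Motion player Blueprint that lets the player select option objects by touching them with an index finger.
; BeginPlay enables swipe gestures on the Leap controller and snaps hand and index-finger collision spheres to sockets on the mesh.
; Overlaps on either fingertip sphere call AttemptToSelectOption, which casts the other actor to option and calls Select.
; The hand spheres and swipe gesture have no handlers in this graph.
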(event `self.ReceiveBeginPlay`
  (`parent.ReceiveBeginPlay`)
  (`LeapController.EnableGesture` (`self.LeapController`) "GESTURE_TYPE_SWIPE" true)
  (`|ExecutionSequence`
    (:`then_0`
      (`SceneComponent.K2_AttachTo` (`self.leftHandCollisionSphere`) (`self.Mesh`) "hand_l_socket" "SnapToTarget" true)
      (`SceneComponent.K2_AttachTo` (`self.rightHandCollisionSphere`) (`self.Mesh`) "hand_r_socket" "SnapToTarget" true))
    (:`then_1`
      (`SceneComponent.K2_AttachTo` (`self.leftIndexFinderCollisionSphere`) (`self.Mesh`) "index_l_socket" "SnapToTarget" true)
      (`SceneComponent.K2_AttachTo` (`self.rightIndexFinderCollisionSphere`) (`self.Mesh`) "index_r_socket" "SnapToTarget" true))))

(event `Key|LeapRightGrab`
  (params (Key :type "Key Structure" :default "AnyKey")))

(event `Key|LeapLeftGrab`
  (params (Key :type "Key Structure" :default "AnyKey")))

(event `self.leftIndexFinderCollisionSphere.OnComponentBeginOverlap`
  (params (OtherActor :type "Actor Object Reference") (OtherComp :type "PrimitiveComponent Object Reference") (OtherBodyIndex :type Integer) (bFromSweep :type Boolean) (SweepResult :type "HitResult Structure (by ref)"))
  (`self.AttemptToSelectOption` OtherActor))

(event `self.rightIndexFinderCollisionSphere.OnComponentBeginOverlap`
  (params (OtherActor :type "Actor Object Reference") (OtherComp :type "PrimitiveComponent Object Reference") (OtherBodyIndex :type Integer) (bFromSweep :type Boolean) (SweepResult :type "HitResult Structure (by ref)"))
  (`self.AttemptToSelectOption` OtherActor))

(fn `UserConstructionScript`
  (`parent.UserConstructionScript`))