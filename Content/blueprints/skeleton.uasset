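; Skeleton actor for an organ-placement activity that highlights organs put in their matching body slots.
; Brain, lungs, stomach and liver boxes each pass overlap begin and end events to a shared check with their expected organ type.
; The check casts the overlapping actor to an organ and compares its Type.
; On a match, its container material switches to a grass material while inside and back to the default on exit.
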(event `self.ReceiveBeginPlay`)

(event `self.ReceiveActorBeginOverlap`
  (params (OtherActor :type "Actor Object Reference")))

(event `self.ReceiveTick`
  (params (DeltaSeconds :type "Float (single-precision)")))

(event `self.brainBox.OnComponentBeginOverlap`
  (params (OtherActor :type "Actor Object Reference") (OtherComp :type "PrimitiveComponent Object Reference") (OtherBodyIndex :type Integer) (bFromSweep :type Boolean) (SweepResult :type "HitResult Structure (by ref)"))
  (`self.CheckOrganAndSetColor` OtherActor "NewEnumerator0" true))

(event `self.brainBox.OnComponentEndOverlap`
  (params (OtherActor :type "Actor Object Reference") (OtherComp :type "PrimitiveComponent Object Reference") (OtherBodyIndex :type Integer))
  (`self.CheckOrganAndSetColor` OtherActor "NewEnumerator0"))

(event `self.lungsBox.OnComponentBeginOverlap`
  (params (OtherActor :type "Actor Object Reference") (OtherComp :type "PrimitiveComponent Object Reference") (OtherBodyIndex :type Integer) (bFromSweep :type Boolean) (SweepResult :type "HitResult Structure (by ref)"))
  (`self.CheckOrganAndSetColor` OtherActor "NewEnumerator3" true))

(event `self.lungsBox.OnComponentEndOverlap`
  (params (OtherActor :type "Actor Object Reference") (OtherComp :type "PrimitiveComponent Object Reference") (OtherBodyIndex :type Integer))
  (`self.CheckOrganAndSetColor` OtherActor "NewEnumerator3"))

(event `self.stomachBox.OnComponentBeginOverlap`
  (params (OtherActor :type "Actor Object Reference") (OtherComp :type "PrimitiveComponent Object Reference") (OtherBodyIndex :type Integer) (bFromSweep :type Boolean) (SweepResult :type "HitResult Structure (by ref)"))
  (`self.CheckOrganAndSetColor` OtherActor "NewEnumerator1" true))

(event `self.stomachBox.OnComponentEndOverlap`
  (params (OtherActor :type "Actor Object Reference") (OtherComp :type "PrimitiveComponent Object Reference") (OtherBodyIndex :type Integer))
  (`self.CheckOrganAndSetColor` OtherActor "NewEnumerator1"))

(event `self.liverBox.OnComponentBeginOverlap`
  (params (OtherActor :type "Actor Object Reference") (OtherComp :type "PrimitiveComponent Object Reference") (OtherBodyIndex :type Integer) (bFromSweep :type Boolean) (SweepResult :type "HitResult Structure (by ref)"))
  (`self.CheckOrganAndSetColor` OtherActor "NewEnumerator2" true))

(event `self.liverBox.OnComponentEndOverlap`
  (params (OtherActor :type "Actor Object Reference") (OtherComp :type "PrimitiveComponent Object Reference") (OtherBodyIndex :type Integer))
  (`self.CheckOrganAndSetColor` OtherActor "NewEnumerator2"))

(fn `CheckOrganAndSetColor`
  (params (object :type "Object Object Reference") (expectedOrganType :type "/Game/blueprints/organType Enum") (shouldSetCorrectColor :type Boolean))
  (bind _organ (`self.IsOrganType` object expectedOrganType)
    (:`True`
      (`self.SetColor` shouldSetCorrectColor _organ))))

(fn `SetColor`
  (params (correctColor :type Boolean) (organ :type "/Game/blueprints/organ Object Reference"))
  (bind _organcontainer (`/Game/blueprints/organ.organContainer` organ))
  (if correctColor
    (`PrimitiveComponent.SetMaterial` _organcontainer 0 "/Game/StarterContent/Materials/M_Ground_Grass.M_Ground_Grass")
    (else
      (`PrimitiveComponent.SetMaterial` _organcontainer 0 "/Game/StarterContent/Props/defaultMat.defaultMat"))))

(fn `UserConstructionScript`)