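; Option is a selectable menu entry that shows an organ type as dash-prefixed text.
; SetOrganType stores the enum and writes its name to the text.
; Set Valid and Set Invalid swap the text material to mark the entry's state, reusing grass and copper materials as indicators.
; Select fires the Selected dispatcher with the organ type and the option itself, and the event graph is empty.
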(event `self.ReceiveBeginPlay`)

(event `self.ReceiveActorBeginOverlap`
  (params (OtherActor :type "Actor Object Reference")))

(event `self.ReceiveTick`
  (params (DeltaSeconds :type "Float (single-precision)")))

(fn `Select`
  (`self.Selected` (`self.organType`) self))

(fn `Set Invalid`
  (`TextRenderComponent.SetTextMaterial` "/Game/StarterContent/Materials/M_Metal_Copper.M_Metal_Copper"))

(fn `Set Valid`
  (`TextRenderComponent.SetTextMaterial` "/Game/StarterContent/Materials/M_Ground_Grass.M_Ground_Grass"))

(fn `SetOrganType`
  (params (type :type "/Game/blueprints/organType Enum"))
  (bind _output_get (set `self.organType` type))
  (`TextRenderComponent.K2_SetText` (`KismetTextLibrary.Conv_StringToText` (`KismetStringLibrary.Concat_StrStr` "- " (`|GetEnumeratorNameAsString` _output_get)))))

(fn `UserConstructionScript`)