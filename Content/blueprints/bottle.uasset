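; Bottle actor for an organ quiz that spawns and attaches an organ of its configured mesh and type at BeginPlay.
; It listens to its child question actor's option selection and marks the option valid or invalid by organ type.
; A valid pick toggles the bottle open or closed through one timeline, played or reversed, that rotates the cover and moves the organ vertically.
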(event `self.ReceiveBeginPlay`
  (bind _returnvalue (`|SpawnActorFromClass` "/Game/blueprints/organ.organ_C" (`self.organTransform`) "Undefined" "OverrideRootScale" null (`self.organMesh`) (`self.organType`)))
  (bind _output_get (set `self.organ` _returnvalue))
  (`self.K2_AttachRootComponentToActor` _output_get self "None" "KeepRelativeOffset" true)
  (bind _asquestion (cast `/Game/blueprints/question` (`ChildActorComponent.ChildActor` (`self.question`))))
  (add `/Game/blueprints/question.Option Selected` _asquestion (delegate `Option Selected Handler`)))

(event `Option Selected Handler`
  (params (organType :type "/Game/blueprints/organType Enum") (option :type "/Game/blueprints/option Object Reference"))
  (if (`|EnumEquality` organType (`self.organType`))
    (`/Game/blueprints/option.Set Valid` option)
    (`self.ToggleOpenClose`)
    (else
      (`/Game/blueprints/option.Set Invalid` option))))

(event `self.ReceiveActorBeginOverlap`
  (params (OtherActor :type "Actor Object Reference")))

(event `self.ReceiveTick`
  (params (DeltaSeconds :type "Float (single-precision)")))

(event `ToggleOpenClose`
  (set `self.openCloseAnimationRunning` true)
  (if (`self.isOpen`)
    (set `self.isOpen` false)
    (bind (_direction _cover_rotation _organlocation) (`Timeline|Timeline_0` :!via `Reverse` :!label _label)
      (:`Update`
        (`SceneComponent.K2_SetRelativeRotation` (`self.cover`) (`KismetMathLibrary.MakeRotator` 0.0 _cover_rotation 0.0) false false)
        (`self.K2_SetActorRelativeLocation` (`self.organ`) (`KismetMathLibrary.MakeVector` 0.0 0.0 _organlocation) false false))
      (:`Finished`
        (set `self.openCloseAnimationRunning` false)))
    (else
      (set `self.isOpen` true)
      (goto _label))))

(event `self.ReceiveActorBeginOverlap`
  (params (OtherActor :type "Actor Object Reference")))

(event `self.ReceiveActorEndOverlap`
  (params (OtherActor :type "Actor Object Reference")))

(fn `ReturnChild`
  (returns (ReturnValue :type "SceneComponent Object Reference"))
  (return null))

(fn `UserConstructionScript`)